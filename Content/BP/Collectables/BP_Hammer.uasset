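; BP_Hammer is a collectable hammer that, on interaction, destroys itself, notifies breakable doors and shows a collected widget.
; It calls CollectHammer on the BP_BreakableDoor actors found in the level after running the parent Interact.
; A sphere overlap toggles the prompt widget, while Tick spins the pivot and IdleAnim plays a timeline that bobs it vertically.
; A scene capture component renders only the hammer mesh; the older tutorial-text sequence is disconnected.
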(event OnComponentBeginOverlap(Sphere)
  (params (OverlappedComponent :type Primitive%20Component%20Object%20Reference) (OtherActor :type Actor%20Object%20Reference) (OtherComp :type Primitive%20Component%20Object%20Reference) (OtherBodyIndex :type Integer) (bFromSweep :type Boolean) (SweepResult :type Hit%20Result%20Structure%20%28by%20ref%29))
  ;[1 1 1] Interact Prompt
  (Rendering|SetVisibility (Variables|Default|GetWidget) true false))

(event OnComponentEndOverlap(Sphere)
  (params (OverlappedComponent :type Primitive%20Component%20Object%20Reference) (OtherActor :type Actor%20Object%20Reference) (OtherComp :type Primitive%20Component%20Object%20Reference) (OtherBodyIndex :type Integer))
  ;[1 1 1] Interact Prompt
  (Rendering|SetVisibility (Variables|Default|GetWidget) false false))

(event Custom|IdleAnim
  (bind _zmovement (Timeline|TimelineIdle Play)
    (:Update
      (Transformation|SetRelativeLocation (Variables|Default|GetPivot) (Math|Vector|MakeVector 0.0 0.0 (* _zmovement (Variables|Default|GetAnim_ZDist))) false false))))

(event EventInteract
  (params (Other%20Actor :type Actor%20Object%20Reference))
  ;[1 1 1] Hammer Breaking Code + Dialog
  (|CallParentFunction Other%20Actor)
  (Actor|DestroyActor)
  (bind _outactors (Actor|GetAllActorsOfClass "/Game/BP/Plattform/BP_BreakableDoor.BP_BreakableDoor_C"))
  (Default|CollectHammer _outactors)
  (bind _returnvalue (UserInterface|CreateWidget "/Game/UI/BPW_HammerCollected.BPW_HammerCollected_C"))
  (UserInterface|Viewport|AddtoViewport _returnvalue 0))

(event EventTick
  (params (DeltaSeconds :type Float%20%28single-precision%29))
  (Transformation|AddRelativeRotation (Variables|Default|GetPivot) (Math|Rotator|MakeRotator 0.0 0.0 (* (Variables|Default|GetIdle_RotSpeed) (Utilities|Time|GetWorldDeltaSeconds))) false false))

(event EventBeginPlay
  (Rendering|SceneCapture|ShowOnlyComponent (Variables|Default|GetSceneCaptureComponent2D) (Variables|Default|GetHammer)))

(fn ConstructionScript)

(fn IsPickedUp
  (return (== (Variables|Default|GetHammerPickedUp) 1)))