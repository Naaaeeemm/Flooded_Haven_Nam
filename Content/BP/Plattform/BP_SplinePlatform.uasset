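; BP_SplinePlatform is a platform actor that travels along the spline of a referenced SplineActor when hit.
; It snaps to the spline start on BeginPlay, and Hit triggers a Timeline whose play rate derives from TimeToCompleteInSec.
; Each update maps the track value to a world-space distance along the spline.
; A DoOnce blocks retriggering until the Timeline finishes; WallBroken is an empty stub.
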(event Custom|WallBroken)

(event Custom|Move%20Object
  (Components|Timeline|SetPlayRate (Variables|Default|GetTimeline) (/ 1.0 (Variables|Default|GetTimeToComplete%28inSec%29)))
  (Utilities|FlowControl|DoOnce false
    (:Completed
      (bind _movetrack (Timeline|Timeline PlayFromStart)
        (:Update
          (CallFunction|SetLocationAlongSpline _movetrack))
        (:Finished
          (CallFunction|ResetMove))))))

(event Custom|ResetMove
  (Utilities|FlowControl|DoOnce false) ; enters at Reset
)

(event EventBeginPlay
  (CallFunction|SetLocationAlongSpline 0.0))

(event Collision|EventHit
  (params (MyComp :type Primitive%20Component%20Object%20Reference) (Other :type Actor%20Object%20Reference) (OtherComp :type Primitive%20Component%20Object%20Reference) (bSelfMoved :type Boolean) (HitLocation :type Vector :default "0, 0, 0") (HitNormal :type Vector :default "0, 0, 0") (NormalImpulse :type Vector :default "0, 0, 0") (Hit :type Hit%20Result%20Structure%20%28by%20ref%29))
  (CallFunction|MoveObject))

(fn ConstructionScript)

(fn SetLocationAlongSpline
  (params (Percentage :type Float%20%28double-precision%29))
  (Transformation|SetActorTransform (Math|Transform|MakeTransform (Spline|GetLocationatDistanceAlongSpline (Variables|/Game/BP/Plattform/BP_SplineActor.BP_SplineActor_C|GetSpline (Variables|Default|GetSplineActor)) (Math|Float|Lerp 0.0 (Spline|GetSplineLength (Variables|/Game/BP/Plattform/BP_SplineActor.BP_SplineActor_C|GetSpline (Variables|Default|GetSplineActor))) Percentage) "World") (Math|Rotator|MakeRotator 0.0 0.0 0.0) "1.000000,1.000000,1.000000")))