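; BP_BreakableDoor is an interactable door that the player can break only after collecting a hammer.
; CollectHammer sets the HasHammer flag, and Interact then destroys the door, or otherwise briefly shows a no-hammer message through the character's TutorialText UI.
; Sphere overlap toggles the door's widget.
; OpenDoor is empty, and older counter, breaking-toggle and scale logic remains unconnected.
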(event OnComponentBeginOverlap(Sphere)
  (params (OverlappedComponent :type Primitive%20Component%20Object%20Reference) (OtherActor :type Actor%20Object%20Reference) (OtherComp :type Primitive%20Component%20Object%20Reference) (OtherBodyIndex :type Integer) (bFromSweep :type Boolean) (SweepResult :type Hit%20Result%20Structure%20%28by%20ref%29))
  (Rendering|SetVisibility (Variables|Default|GetWidget) true false))

(event OnComponentEndOverlap(Sphere)
  (params (OverlappedComponent :type Primitive%20Component%20Object%20Reference) (OtherActor :type Actor%20Object%20Reference) (OtherComp :type Primitive%20Component%20Object%20Reference) (OtherBodyIndex :type Integer))
  (Rendering|SetVisibility (Variables|Default|GetWidget) false false))

(event Custom|CollectHammer
  (Variables|Default|SetHasHammer true))

(event Custom|OpenDoor)

(event EventBeginPlay)

(event EventInteract
  (params (Other%20Actor :type Actor%20Object%20Reference))
  (|CallParentFunction Other%20Actor)
  (if (Variables|Default|GetHasHammer)
    (Actor|DestroyActor)
    (else
      (Widget|SetVisibility (Variables|/Game/UI/BPW_TutorialText.BPW_TutorialText_C|GetTextBlock_NoHammer (Variables|/Game/BP/Player/BP_ThirdPersonCharacter.BP_ThirdPersonCharacter_C|GetTutorial%20Text (Variables|Default|GetThirdPersonCharacter))) "Visible")
      (Default|UIVisible (Variables|/Game/BP/Player/BP_ThirdPersonCharacter.BP_ThirdPersonCharacter_C|GetTutorial%20Text (Variables|Default|GetThirdPersonCharacter)))
      (Utilities|FlowControl|Delay 2.0)
      (Widget|SetVisibility (Variables|/Game/UI/BPW_TutorialText.BPW_TutorialText_C|GetTextBlock_NoHammer (Variables|/Game/BP/Player/BP_ThirdPersonCharacter.BP_ThirdPersonCharacter_C|GetTutorial%20Text (Variables|Default|GetThirdPersonCharacter))) "Collapsed")
      (Default|UICollapsed (Variables|/Game/BP/Player/BP_ThirdPersonCharacter.BP_ThirdPersonCharacter_C|GetTutorial%20Text (Variables|Default|GetThirdPersonCharacter))))))

(fn ConstructionScript)

(fn SetScale
  (params (Scale :type Float%20%28double-precision%29))
  (Transformation|SetActorScale3D (Math|Vector|MakeVector Scale Scale 1.0)))