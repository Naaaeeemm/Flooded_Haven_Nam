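; BP_Respawnpoint is a checkpoint actor that becomes the character's respawn point on overlap.
; Overlap by BP_ThirdPersonCharacter stores this actor in the character's MyRespawnPoint every time.
; A DoOnce limits the checkpoint widget, static sound and Pause audio-settings initialization to the first such overlap.
; GetRespawnLocRot exposes the RespawnPivot component's world location and rotation as the respawn transform.
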(event Collision|EventActorBeginOverlap
  (params (OtherActor :type Actor%20Object%20Reference))
  (bind _asbp_third_person_character (Utilities|Casting|CastToBP_ThirdPersonCharacter OtherActor))
  (Variables|/Game/BP/Player/BP_ThirdPersonCharacter.BP_ThirdPersonCharacter_C|SetMyRespawnPoint _asbp_third_person_character self)
  (Utilities|FlowControl|DoOnce false
    (:Completed
      (bind _returnvalue (UserInterface|CreateWidget "/Game/UI/BPW_Checkpoint.BPW_Checkpoint_C"))
      (UserInterface|Viewport|AddtoViewport _returnvalue 0)
      (Audio|PlaySound2D "/Game/Sound/SFX/ES_Tuning_Between_Stations__Static_02_-_Epidemic_Sound_-_1840-3855.ES_Tuning_Between_Stations__Static_02_-_Epidemic_Sound_-_1840-3855" 1.0 1.0 0.0 0 0)
      (Default|InitAudioSettings (Variables|Default|Getpause)))))

(fn ConstructionScript
  (|CallParentFunction))

(fn GetRespawnLocRot
  (bind _respawnpivot (Variables|Default|GetRespawnPivot))
  (return (Transformation|GetWorldLocation _respawnpivot) (Transformation|GetWorldRotation _respawnpivot)))